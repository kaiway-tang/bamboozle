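; BP_PlayerTest is a test player Blueprint that captures raw keyboard and mouse input into variables.
; WASD and left mouse set held-state booleans, mouse axes are stored each update, and Space calls KeySpaceDown, which has no body here.
; Nothing in this graph reads the stored input, and Tick's forward AddForce sits behind an always-false branch, so it never moves anything.
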(event EventBeginPlay)

(event Collision|EventActorBeginOverlap
  (params (OtherActor :type Actor%20Object%20Reference)))

(event EventTick
  (params (DeltaSeconds :type Float%20%28single-precision%29))
  (if false
    (Class|PlayerClone|AddForce (* (Transformation|GetActorForwardVector) 1e+04) true)))

(event Input|MouseEvents|MouseX
  (params (AxisValue :type Float%20%28single-precision%29))
  (Variables|Default|SetmouseX AxisValue))

(event Input|MouseEvents|MouseY
  (params (AxisValue :type Float%20%28single-precision%29))
  (Variables|Default|SetmouseY AxisValue))

(event Input|MouseEvents|LeftMouseButton
  (params (Key :type Key%20Structure :default "None"))
  (:Pressed
    (Variables|Default|SetLMBPressed true))
  (:Released
    (Variables|Default|SetLMBPressed false)))

(event Input|KeyboardEvents|W
  (params (Key :type Key%20Structure :default "None"))
  (:Pressed
    (Variables|Default|SetkeyWDown true))
  (:Released
    (Variables|Default|SetkeyWDown false)))

(event Input|KeyboardEvents|S
  (params (Key :type Key%20Structure :default "None"))
  (:Pressed
    (Variables|Default|SetkeySDown true))
  (:Released
    (Variables|Default|SetkeySDown false)))

(event Input|KeyboardEvents|A
  (params (Key :type Key%20Structure :default "None"))
  (:Pressed
    (Variables|Default|SetkeyADown true))
  (:Released
    (Variables|Default|SetkeyADown false)))

(event Input|KeyboardEvents|D
  (params (Key :type Key%20Structure :default "None"))
  (:Pressed
    (Variables|Default|SetkeyDDown true))
  (:Released
    (Variables|Default|SetkeyDDown false)))

(event Input|KeyboardEvents|SpaceBar
  (params (Key :type Key%20Structure :default "None"))
  (:Pressed
    (Class|PlayerClone|KeySpaceDown)))

(fn ConstructionScript)