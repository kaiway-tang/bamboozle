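; GM_Bamboozle is the game mode Blueprint that handles pawn possession switching and shows the end screen.
; SwitchPosession gets a pawn from CyclePawn, with an optional reverse direction, and has player controller 0 possess it.
; Tick polls the QueueGameUI flag, clears it and calls DisplayEndScreen after a debug print.
; DisplayEndScreen creates WBP_EndScreen, passes it Score, shows the cursor and switches input to UI only.
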(event Custom|Switch%20Posession
  (params (cycleReverse :type Boolean))
  (bind _returnvalue (Class|BamboozleGameMode|CyclePawn cycleReverse))
  (Pawn|Possess (Game|GetPlayerController 0) _returnvalue))

(event Custom|DisplayEndScreen
  (bind _returnvalue (Game|GetPlayerController 0))
  (bind _returnvalue_2 (UserInterface|CreateWidget "/Game/Custom/WBP_EndScreen.WBP_EndScreen_C" _returnvalue))
  (Default|SetScoreString _returnvalue_2 (Variables|Default|GetScore))
  (UserInterface|Viewport|AddtoViewport _returnvalue_2 5)
  (Variables|/Script/Engine.PlayerController|SetbShowMouseCursor _returnvalue true)
  (Input|SetInputModeUIOnly _returnvalue _returnvalue_2 "DoNotLock" false))

(event EventBeginPlay)

(event EventTick
  (params (DeltaSeconds :type Float%20%28single-precision%29))
  (if (Variables|Default|GetQueueGameUI)
    (Development|PrintString "Hello")
    (Variables|Default|SetQueueGameUI false)
    (CallFunction|DisplayEndScreen)))

(fn ConstructionScript)