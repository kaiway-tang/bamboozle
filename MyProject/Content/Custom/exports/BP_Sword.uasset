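; BP_Sword is a Blueprint with a sword component and three decorative or mechanical rings that animate continuously.
; Tick spins the rings about yaw at different rates, with the middle one counter-rotating.
; The MoveSword event snaps the sword down by a given distance along local Z, and Tick raises it back toward zero at RecoverySpeed.
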(event Custom|MoveSword
  (params (UnitsDown :type Float%20%28double-precision%29))
  (Transformation|SetRelativeLocation (Variables|Default|GetSwordRef) (Math|Vector|MakeVector 0.0 0.0 (* UnitsDown -1.0)) false false))

(event EventBeginPlay)

(event Collision|EventActorBeginOverlap
  (params (OtherActor :type Actor%20Object%20Reference)))

(event EventTick
  (params (DeltaSeconds :type Float%20%28single-precision%29))
  (bind _z__yaw_ (Variables|Default|GetZ%20%28Yaw%29))
  (bind _returnvalue (Math|Rotator|MakeRotator 0.0 0.0 _z__yaw_))
  (bind _returnvalue_2 (* _returnvalue DeltaSeconds))
  (Transformation|AddRelativeRotation (Variables|Default|GetRingRef) _returnvalue_2 false false)
  (Transformation|AddRelativeRotation (Variables|Default|GetRingRef1) (* _returnvalue_2 -1.5) false false)
  (Transformation|AddRelativeRotation (Variables|Default|GetRingRef2) (* _returnvalue_2 2.0) false false)
  (if (< (.z (.location (Transformation|GetRelativeTransform (Variables|Default|GetSwordRef)))) 0.0)
    (Transformation|AddRelativeLocation (Variables|Default|GetSwordRef) (Math|Vector|MakeVector 0.0 0.0 (* DeltaSeconds (Variables|Default|GetRecoverySpeed))) false false)))

(fn ConstructionScript)