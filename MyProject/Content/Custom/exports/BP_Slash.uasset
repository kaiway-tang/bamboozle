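; BP_Slash is an actor that plays a left or right slash effect on a static mesh through a scrolling material.
; The construction script creates a dynamic instance of M_Slash, which BeginPlay applies to the mesh.
; QueueSlash sets the direction and resets LerpValue to that side's start point.
; While LerpValue stays within its range, Tick moves it by LerpSpeed and feeds it to the ScrollLerp parameter.
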(event Custom|QueueSlash
  (params (Left :type Boolean))
  (bind _output_get (Variables|Default|SetSlashLeft Left))
  (if _output_get
    (Variables|Default|SetLerpValue 0.7)
    (else
      (Variables|Default|SetLerpValue 0.3))))

(event EventBeginPlay
  (Rendering|Material|SetMaterial (Variables|Default|GetStaticMesh) 0 (Variables|Default|GetDynamicMaterial)))

(event EventTick
  (params (DeltaSeconds :type Float%20%28single-precision%29))
  (bind _lerpspeed (Variables|Default|GetLerpSpeed))
  (bind _returnvalue (* DeltaSeconds _lerpspeed))
  (if (Math|Float|InRange(Float) (Variables|Default|GetLerpValue) 0.0 1.0 false false)
    (if (Variables|Default|GetSlashLeft)
      (Variables|Default|SetLerpValue (- (Variables|Default|GetLerpValue) _returnvalue))
      (else
        (Variables|Default|SetLerpValue (+ (Variables|Default|GetLerpValue) _returnvalue))))
    (Rendering|Material|SetScalarParameterValueonMaterials (Variables|Default|GetStaticMesh) "ScrollLerp" (Variables|Default|GetLerpValue))))

(event Input|MouseEvents|LeftMouseButton
  (params (Key :type Key%20Structure :default "None")))

(fn ConstructionScript
  (bind _returnvalue (Rendering|Material|CreateDynamicMaterialInstance "/Game/Custom/exports/M_Slash.M_Slash" "None" "None" :!class /Script/Engine.KismetMaterialLibrary))
  (Variables|Default|SetDynamicMaterial _returnvalue))